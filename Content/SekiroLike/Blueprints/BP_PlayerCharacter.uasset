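; Player character Blueprint for the SekiroLike game, holding only empty default events and disconnected test snippets.
; BeginPlay, Tick and the construction script do nothing, and the movement and camera rotation comment has no nodes under it.
; The unwired snippets exercise hit-trace toggling, a debug ability-stage gameplay tag, walk/run speed switching, GAS dodge activation and slow motion, but none of them execute.
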(event `self.ReceiveBeginPlay`)

(event `self.ReceiveTick`
  (params (DeltaSeconds :type "Float (single-precision)")))

(event `Key|LeftShift`
  (params (Key :type "Key Structure"))
  ;[0.8621 0.7679 1] 移动和视角旋转
)

(event `Key|LeftMouseButton`
  (params (Key :type "Key Structure")))

(event `Key|LeftAlt`
  (params (Key :type "Key Structure")))

(event `Key|Q`
  (params (Key :type "Key Structure")))

(fn `UserConstructionScript`)