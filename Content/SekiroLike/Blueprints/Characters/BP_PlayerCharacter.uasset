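; Player character Blueprint for a Sekiro-like game; its graph holds little more than debug and test logic.
; Pressing Q applies a damage-immunity Gameplay Effect to itself through its Ability System Component, with the duration overridden on the spec.
; BeginPlay, Tick and the construction script are empty.
; Disconnected test snippets remain for hit tracing, dodge activation, walk/run speed, posture printing, gameplay tags and time dilation.
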(event `self.ReceiveBeginPlay`
  ;[1 0.1875 0] For Debug
)

(event `self.ReceiveTick`
  (params (DeltaSeconds :type "Float (single-precision)"))
  ;[1 0.1875 0] For Debug
)

(event `Key|Q`
  (params (Key :type "Key Structure"))
  (bind _returnvalue (`AbilitySystemBlueprintLibrary.GetAbilitySystemComponent` self))
  (:`Pressed`
    (bind _returnvalue_2 (`AbilitySystemBlueprintLibrary.SetDuration` (`AbilitySystemComponent.MakeOutgoingSpec` _returnvalue "/Game/SekiroLike/Blueprints/Abilities/GameplayEffects/GE_Buff_DamageImmunity.GE_Buff_DamageImmunity_C" 0.0 (`AbilitySystemComponent.MakeEffectContext` _returnvalue)) 10.0))
    (`AbilitySystemComponent.BP_ApplyGameplayEffectSpecToSelf` (`AbilitySystemBlueprintLibrary.GetAbilitySystemComponent` self) _returnvalue_2)))

(event `Key|LeftShift`
  (params (Key :type "Key Structure"))
  ;[0.8621 0.7679 1] 移动和视角旋转
)

(event `Key|LeftMouseButton`
  (params (Key :type "Key Structure")))

(event `Key|LeftAlt`
  (params (Key :type "Key Structure")))

(event `Key|Q`
  (params (Key :type "Key Structure")))

(fn `UserConstructionScript`)