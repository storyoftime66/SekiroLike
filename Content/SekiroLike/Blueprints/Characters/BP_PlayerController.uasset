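; BP_PlayerController is the player controller for a Sekiro-like game, handling the gameplay HUD and the settings screen.
; On BeginPlay it creates UMG_Gameplay, adds it to the viewport, prints a debug string, then calls MeetEliteEnemy on that widget with no enemy set.
; The P key lazily creates UMG_Settings on first press and toggles its visibility on later presses.
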(event `self.ReceiveBeginPlay`
  (`|ExecutionSequence`
    (:`then_0`
      (bind _returnvalue (`|CreateWidget` "/Game/SekiroLike/Blueprints/UMG/UMG_Gameplay.UMG_Gameplay_C" self))
      (bind _output_get (set `self.UMG_Gameplay` _returnvalue))
      (`UserWidget.AddToViewport` _output_get 0)
      (`KismetSystemLibrary.PrintString` "Hello"))
    (:`then_1`
      (`/Game/SekiroLike/Blueprints/UMG/UMG_Gameplay.MeetEliteEnemy` (`self.UMG_Gameplay`) null) ; Enemy为空
    )))

(event `self.ReceivePossess`
  (params (PossessedPawn :type "Pawn Object Reference")))

(event `Key|P`
  (params (Key :type "Key Structure"))
  (:`Pressed`
    (bind _umg_setting (`self.UMG_Setting`)
      (:`then`
        (`/Game/SekiroLike/Blueprints/UMG/UMG_Settings.ToggleVisibility` _umg_setting))
      (:`else`
        (bind _returnvalue (`|CreateWidget` "/Game/SekiroLike/Blueprints/UMG/UMG_Settings.UMG_Settings_C" self))
        (bind _output_get (set `self.UMG_Setting` _returnvalue))
        (`UserWidget.AddToViewport` _output_get 0)))))

(fn `UserConstructionScript`)