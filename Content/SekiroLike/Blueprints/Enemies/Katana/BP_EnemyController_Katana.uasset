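; AI controller for the katana enemy that runs its behavior tree and supplies it with the player as a target.
; A perception update for a PlayerCharacter stores that actor in the Blackboard and sets the KeyKeep flag.
; It then disables the sight sense, so acquisition is one-way: nothing here clears the target or re-enables sight.
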(event `self.ReceiveBeginPlay`
  (`self.RunBehaviorTree` "/Game/SekiroLike/Blueprints/Enemies/Katana/BT_Enemy_Katana.BT_Enemy_Katana"))

(event `self.AIPerception.OnTargetPerceptionUpdated`
  (params (Actor :type "Actor Object Reference") (Stimulus :type "AIStimulus Structure"))
  (bind _asplayer_character (cast `PlayerCharacter` Actor))
  (`BlackboardComponent.SetValueAsObject` (`AIBlueprintHelperLibrary.GetBlackboard` null) (`self.Key_PlayerActor`) _asplayer_character)
  (`BlackboardComponent.SetValueAsBool` (`AIBlueprintHelperLibrary.GetBlackboard` null) (`self.Key_Keep`) true)
  (`AIPerceptionComponent.SetSenseEnabled` (`self.AIPerception`) "/Script/AIModule.AISense_Sight" false))

(fn `UserConstructionScript`)