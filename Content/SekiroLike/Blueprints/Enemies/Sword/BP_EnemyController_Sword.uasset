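; BP_EnemyController_Sword is the AI controller for the sword enemy in a Sekiro-like game.
; On possess it runs BT_Enemy_Sword and, if that succeeds, waits one second before storing player pawn 0 in the blackboard as the player character.
; Every tick it writes the frame's delta seconds to a float blackboard key.
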(event `self.ReceiveTick`
  (params (DeltaSeconds :type "Float (single-precision)"))
  (`BlackboardComponent.SetValueAsFloat` (`AIBlueprintHelperLibrary.GetBlackboard` null) (`self.Key Name`) DeltaSeconds))

(event `self.ReceivePossess`
  (params (PossessedPawn :type "Pawn Object Reference"))
  (bind _returnvalue (`self.RunBehaviorTree` "/Game/SekiroLike/Blueprints/Enemies/Sword/BT_Enemy_Sword.BT_Enemy_Sword"))
  (if _returnvalue
    (`KismetSystemLibrary.Delay` 1.0)
    (`BlackboardComponent.SetValueAsObject` (`AIBlueprintHelperLibrary.GetBlackboard` null) (`self.Key_PlayerCharacter`) (`GameplayStatics.GetPlayerPawn` 0))))

(fn `UserConstructionScript`)